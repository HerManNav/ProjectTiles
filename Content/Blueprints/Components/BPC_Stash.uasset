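; Actor component that acts as a capped stash of tiles for its owner.
; It keeps a Tiles array limited by MaxTiles: AddTileToStash appends a tile and reports whether it fit, and CanGrabTile reports whether space remains.
; It has no event logic and no removal function, so it works only when other code calls it.
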(event EventBeginPlay)

(event EventTick
  (params (DeltaSeconds :type Float%20%28single-precision%29)))

(fn AddTiletoStash
  (params (Tile :type BPC%20Tile%20BASE%20Object%20Reference%20%28by%20ref%29))
  (if (< (Utilities|Array|Length (Variables|Default|GetTiles)) (Variables|Default|GetMaxTiles))
    (Utilities|Array|Add (Variables|Default|GetTiles) Tile)
    (return true)
    (else
      (return false))))

(fn CanGrabTile
  (return (< (Utilities|Array|Length (Variables|Default|GetTiles)) (Variables|Default|GetMaxTiles))))