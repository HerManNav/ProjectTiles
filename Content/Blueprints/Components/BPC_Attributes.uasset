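; BPC_Attributes is a Blueprint component that tracks health and death state.
; Health resets to MaxHealth and the death flag clears on BeginPlay through ResetHealth.
; ReceiveDamage subtracts damage without clamping and sets IsDead once Health reaches zero or below.
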(event EventBeginPlay
  (CallFunction|ResetHealth))

(event EventTick
  (params (DeltaSeconds :type Float%20%28single-precision%29)))

(fn ReceiveDamage
  (params (Damage :type Float%20%28double-precision%29))
  (bind _output_get (Variables|Health|SetHealth (- (Variables|Health|GetHealth) Damage)))
  (if (<= _output_get 0.0)
    (Variables|Health|SetIsDead true)))

(fn ResetHealth
  (Variables|Health|SetHealth (Variables|Health|GetMaxHealth))
  (Variables|Health|SetIsDead false))