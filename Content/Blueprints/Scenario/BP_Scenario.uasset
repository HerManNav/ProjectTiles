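; BP_Scenario procedurally builds a random tile-based level at BeginPlay from tile components added at runtime under BasePosition.
; Probability rolls place bridge basement and rock ground along X, filtered by ShouldGenerateTileAtPosition, then paired rock back walls at both edges.
; Both side playgrounds get capped runs of platform tiles, with row odds cut tenfold after a hit and recomputed from height after a miss.
; Grab destroys a tile and its child components.
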(event EventBeginPlay
  (bind _numberoftilesx (Variables|Default|GetNumberOfTilesX))
  (Utilities|FlowControl|Sequence
    (:then_0
      (for _index (range 0 (Variables|Default|GetNumberOfTilesX))
        (if (|ShouldGenerateTileAtPosition _index)
          (Basement|TryCreateBasementTile _index)
          (MainTiles|TryCreateMainGround _index))))
    (:then_1
      (MainTiles|TryCreateBackWalls))
    (:then_2
      (Playground|TryCreatePlayground 1 (Variables|Generator|Playground|GetPlaygroundsExtension))
      (Playground|TryCreatePlayground (- _numberoftilesx (Variables|Generator|Playground|GetPlaygroundsExtension)) (Utilities|Operators|Subtract _numberoftilesx 1 1)))))

(event EventGrab
  (params (Tile :type BPC%20Tile%20BASE%20Object%20Reference))
  (Utilities|FlowControl|Sequence
    (:then_0
      (for _array_element (Components|GetChildrenComponents Tile true)
        (Components|DestroyComponent _array_element)))
    (:then_1
      (Components|DestroyComponent Tile))))

(fn ConstructionScript)

(fn DestroyTile
  (params (TileComponent :type Paper%20Tile%20Map%20Component%20Object%20Reference))
  (Components|DestroyComponent TileComponent))

(fn CreateNewTile
  (params (NewTileMap :type BPC%20Tile%20BASE%20Class%20Reference) (X :type Integer) (Z :type Integer))
  (bind _tilesize (Variables|Default|GetTileSize))
  (bind _returnvalue (Game|AddComponentbyClass NewTileMap false (Math|Transform|MakeTransform (Math|Vector|MakeVector (Math|Conversions|ToFloat(Integer) (* X _tilesize)) 0.0 (Math|Conversions|ToFloat(Integer) (* Z _tilesize))) "0, 0, 0" "1.000000,1.000000,1.000000")))
  (Transformation|AttachComponentToComponent _returnvalue (Variables|Default|GetBasePosition) "None" "KeepRelative" "KeepRelative" "KeepRelative" true))

(fn TryCreateBasementTile
  (params (X :type Integer))
  (if (< (Math|Random|RandomFloat) (Variables|Generator|Basement|GetBasementGenerationProbability))
    (General|CreateNewTile "/Game/Blueprints/Components/Tiles/Regular/Types/BPC_Tile_Regular_Bridge.BPC_Tile_Regular_Bridge_C" X (Variables|Generator|Basement|GetBasementZ))))

(fn TryCreateMainGround
  (params (X :type Integer))
  (if (< (Math|Random|RandomFloat) (Variables|Generator|MainGround|GetMainGroundGenerationProbability))
    (General|CreateNewTile "/Game/Blueprints/Components/Tiles/Regular/Types/BPC_Tile_Regular_Rock.BPC_Tile_Regular_Rock_C" X (Variables|Generator|MainGround|GetMainGroundZ))))

(fn TryCreateBackWalls
  (for _index (range (+ (Variables|Generator|MainGround|GetMainGroundZ) 1) (Variables|Generator|BackWalls|GetBackWallsHighestZ))
    (if (< (Math|Random|RandomFloat) (Variables|Generator|BackWalls|GetBackWallsGenerationProbability))
      (General|CreateNewTile "/Game/Blueprints/Components/Tiles/Regular/Types/BPC_Tile_Regular_Rock.BPC_Tile_Regular_Rock_C" 0 _index)
      (General|CreateNewTile "/Game/Blueprints/Components/Tiles/Regular/Types/BPC_Tile_Regular_Rock.BPC_Tile_Regular_Rock_C" (Variables|Generator|BackWalls|GetBackWallsRightmostColumn) _index))))

(fn TryCreatePlayground
  (params (MinX :type Integer) (MaxX :type Integer))
  (bind _maingroundz (Variables|Generator|MainGround|GetMainGroundZ))
  (bind _playgroundsbaserowovermainground (Variables|Default|GetPlaygroundsBaseRowOverMainGround))
  (bind _returnvalue (+ _maingroundz _playgroundsbaserowovermainground))
  ;[1 1 1] Row selection
  (for _index (range _returnvalue (Variables|Generator|Playground|GetPlaygroundsHighestRow))
    (LocalVariables|SetCurrentRow _index)
    (if (< (Math|Random|RandomFloat) (Variables|Generator|Playground|GetPlaygroundsRowGenerationProbability))
      (bind _output_get (Variables|Generator|Playground|SetPlaygroundsRowGenerationProbability (/ (stale _output_get) 1e+01)))
      ;[1 1 1] Column selection
      (Variables|Generator|Playground|SetPlaygroundsColumnCounter MinX)
      (Variables|Generator|Playground|SetPlaygroundsRowGeneratedTiles 0)
      (bind _index_2 (Utilities|FlowControl|ForLoopwithBreak MinX MaxX :!label _label)
        (:LoopBody
          (if (and (>= _index_2 (Variables|Generator|Playground|GetPlaygroundsColumnCounter)) (< (Math|Random|RandomFloat) (Variables|Generator|Playground|GetPlaygroundsColumnGenerationProbability)))
            (bind _output_get_2 (Variables|Generator|Playground|SetPlaygroundsColumnCounter (+ (stale _output_get_2) (Math|Random|RandomIntegerinRange 2 6))))
            (for _index_3 (range _index_2 (Math|Integer|Min(Integer) MaxX _output_get_2))
              (if (<= (Variables|Generator|Playground|GetPlaygroundsRowGeneratedTiles) (Variables|Generator|Playground|GetPlaygroundsMaxTilesPerRow))
                (General|CreateNewTile "/Game/Blueprints/Components/Tiles/Regular/Types/BPC_Tile_Regular_Platform.BPC_Tile_Regular_Platform_C" _index_3 (LocalVariables|GetCurrentRow))
                (Math|Integer|IncrementInt (Variables|Generator|Playground|GetPlaygroundsRowGeneratedTiles))
                (else
                  (goto _label Break))))
            (elif (<= (Variables|Generator|Playground|GetPlaygroundsColumnCounter) _index_2)
              (bind _output_get_3 (Variables|Generator|Playground|SetPlaygroundsColumnCounter (+ (stale _output_get_3) 1)))))))
      (else
        (bind _output_get_4 (Variables|Generator|Playground|SetPlaygroundsRowGenerationProbability (|((prob+0.200000)*(currentHeight/baseHeight)) (stale _output_get_4) (Math|Conversions|ToFloat(Integer) _index) (Math|Conversions|ToFloat(Integer) _returnvalue))))))))