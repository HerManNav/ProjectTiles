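; Base 2D sprite action character that handles damage, hit feedback, bullet energy and contact with pushing objects.
; Damage goes to BPCAttributes, notifies of the hit, then either signals defeat or triggers a flash.
; The flash uses a timeline with a swappable curve to fade emissive intensity on the sprite's dynamic material.
; Bullet-destroyed notifications update clamped bullet energy, and overlapping a BP_PushingObject adds forced movement input along its forward vector.
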(event OnComponentBeginOverlap(CapsuleComponent)
  (params (OverlappedComponent :type Primitive%20Component%20Object%20Reference) (OtherActor :type Actor%20Object%20Reference) (OtherComp :type Primitive%20Component%20Object%20Reference) (OtherBodyIndex :type Integer) (bFromSweep :type Boolean) (SweepResult :type Hit%20Result%20Structure%20%28by%20ref%29))
  (CallFunction|OnRootComponentBeginOverlap OverlappedComponent OtherActor OtherComp))

(event Custom|Flash
  (params (Intensity :type Float%20%28single-precision%29) (PlayRate :type Float%20%28single-precision%29) (Color :type Linear%20Color%20Structure :default "(R=1.000000,G=0.822786,B=0.124772,A=1.000000)") (Curve :type Curve%20Float%20Object%20Reference))
  (bind _dynamicmatinst (Variables|Flash|GetDynamicMatInst))
  (bind _flashtimeline (Variables|Default|GetFlashTimeline))
  ;[1 1 1] Damage
  (Rendering|Material|SetVectorParameterValue _dynamicmatinst "EmissiveColor" Color :!class /Script/Engine.MaterialInstanceDynamic)
  (Rendering|Material|SetScalarParameterValue _dynamicmatinst "EmissiveIntensity" Intensity :!class /Script/Engine.MaterialInstanceDynamic)
  (Class|TimelineComponent|SetFloatCurve _flashtimeline Curve "Alpha")
  (Components|Timeline|SetPlayRate _flashtimeline PlayRate)
  (bind _alpha (Timeline|FlashTimeline PlayFromStart)
    (:Update
      (Rendering|Material|SetScalarParameterValue _dynamicmatinst "EmissiveIntensity" (Math|Float|Lerp Intensity 0.0 _alpha) :!class /Script/Engine.MaterialInstanceDynamic))))

(event Custom|OnRootComponentBeginOverlap
  (params (OveralappedComponent :type Primitive%20Component%20Object%20Reference) (OtherActor :type Actor%20Object%20Reference) (OtherComponent :type Primitive%20Component%20Object%20Reference))
  ;[1 1 1] Pushing objects
  (bind _asbp_pushing_object (Utilities|Casting|CastToBP_PushingObject OtherActor))
  (Pawn|Input|AddMovementInput (Variables|/Game/Blueprints/Props/PushingObjects/BP_PushingObject.BP_PushingObject_C|GetForwardVector _asbp_pushing_object) 1.0 true))

(event Game|Damage|EventAnyDamage
  (params (Damage :type Float%20%28single-precision%29) (DamageType :type Damage%20Type%20Object%20Reference) (InstigatedBy :type Controller%20Object%20Reference) (DamageCauser :type Actor%20Object%20Reference))
  (bind _bpc_attributes (Variables|Default|GetBPC_Attributes))
  ;[1 1 1] Damage
  (Default|ReceiveDamage _bpc_attributes Damage)
  (Default|CallPlayerHit Damage)
  (if (Variables|/Game/Blueprints/Components/BPC_Attributes.BPC_Attributes_C|GetIsDead _bpc_attributes)
    (Default|CallCharacterDefeated)
    (else
      (CallFunction|Flash (Variables|Flash|Damage|GetFlashIntensity) (Variables|Flash|Damage|GetFlashTimelinePlayRate) (Variables|Flash|Damage|GetHitFlashColor)))))

(event EventBeginPlay
  (Development|SetHiddeninGame (Variables|Default|GetCapsuleComponent) (not (Variables|Default|GetbShowDebugCapsules)) false)
  (bind _returnvalue (Rendering|Material|CreateDynamicMaterialInstance (Variables|Default|GetSprite) 0 0 "None" :!class /Script/Engine.PrimitiveComponent))
  (Variables|Flash|SetDynamicMatInst _returnvalue))

(event EventNotifyBulletAbouttobeDestroyed
  (params (BulletEnergy :type Float%20%28double-precision%29))
  (Variables|Shoot|Energy|SetBulletEnergy (Math|Float|Clamp(Float) (+ BulletEnergy (Variables|Shoot|Energy|GetBulletEnergy)) 0.0 (Variables|Shoot|Energy|GetMaxBulletEnergy))))

(fn ConstructionScript
  (Rendering|Material|SetMaterial (Variables|Default|GetSprite) 0 "/Game/Materials/MI_UnlitSprite.MI_UnlitSprite"))