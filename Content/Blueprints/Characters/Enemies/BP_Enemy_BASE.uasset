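; Base enemy character Blueprint that handles defeat, death effects and position reset for enemies.
; On BeginPlay it stores its starting transform and binds to the CharacterDefeated dispatcher, destroying itself when that fires.
; The Destroyed event spawns an explosion actor at its location, so the effect plays on any destruction, not only defeat.
; ResetEnemyTransform teleports the enemy back to the stored transform without sweeping.
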(event Custom|OnCharacterDefeated
  (Actor|DestroyActor))

(event EventBeginPlay
  (|CallParentFunction)
  (Variables|Default|SetOriginalTransform (Transformation|GetActorTransform))
  (EventDispatchers|AssignCharacterDefeated (delegate Custom|OnCharacterDefeated)))

(event EventDestroyed
  (CallFunction|PlayDieVFX))

(fn ConstructionScript
  (|CallParentFunction))

(fn PlayDieVFX
  (Game|SpawnActorfromClass "/Game/Blueprints/VFX/BP_Explosion_EnemyDie.BP_Explosion_EnemyDie_C" (Math|Transform|MakeTransform (Transformation|GetActorLocation) (Transformation|GetActorRotation) "1.000000,1.000000,1.000000") "AlwaysSpawn" "MultiplyWithRoot" 0 0))

(fn ResetEnemyTransform
  (Transformation|SetActorTransform (Variables|Default|GetOriginalTransform) false true))