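; Base projectile actor that damages action characters of a different faction from its owner's.
; Sphere overlaps with those characters apply damage, then destroy it and spawn an explosion; blocking hits do the same without damage.
; A throttled Tick destroys it once it leaves the viewport horizontally, checked by screen projection.
; Any destruction plays a sound and notifies the owner through BPI_Shoot, passing the damage value.
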(event OnComponentHit(Sphere)
  (params (HitComponent :type Primitive%20Component%20Object%20Reference) (OtherActor :type Actor%20Object%20Reference) (OtherComp :type Primitive%20Component%20Object%20Reference) (NormalImpulse :type Vector :default "0, 0, 0") (Hit :type Hit%20Result%20Structure%20%28by%20ref%29))
  ;[1 1 1] Hit & overlaps
  (Actor|DestroyActor)
  (CallFunction|PlayExplosionVFX))

(event OnComponentBeginOverlap(Sphere)
  (params (OverlappedComponent :type Primitive%20Component%20Object%20Reference) (OtherActor :type Actor%20Object%20Reference) (OtherComp :type Primitive%20Component%20Object%20Reference) (OtherBodyIndex :type Integer) (bFromSweep :type Boolean) (SweepResult :type Hit%20Result%20Structure%20%28by%20ref%29))
  ;[1 1 1] Hit & overlaps
  (bind _asbp_action_character_base (Utilities|Casting|CastToBP_ActionCharacter_BASE OtherActor))
  (if (Utilities|Enum|NotEqual(Enum) (Variables|Default|GetOwnerFaction) (Variables|/Game/Blueprints/Characters/BP_ActionCharacter_BASE.BP_ActionCharacter_BASE_C|GetFaction _asbp_action_character_base))
    (Utilities|FlowControl|Sequence
      (:then_0
        (Game|Damage|ApplyDamage _asbp_action_character_base (Variables|Default|GetDamage) 0 self))
      (:then_1
        (Actor|DestroyActor)
        (CallFunction|PlayExplosionVFX)))))

(event EventBeginPlay
  ;[1 1 1] BeginPlay & Destroy
  (bind _asbp_action_character_base (Utilities|Casting|CastToBP_ActionCharacter_BASE (Components|GetOwner)))
  (Variables|Default|SetOwnerFaction (Variables|/Game/Blueprints/Characters/BP_ActionCharacter_BASE.BP_ActionCharacter_BASE_C|GetFaction _asbp_action_character_base)))

(event EventDestroyed
  ;[1 1 1] BeginPlay & Destroy
  (Audio|PlaySoundatLocation "/Game/Audio/SFX/BulletsDestroyed_Cue.BulletsDestroyed_Cue" (Transformation|GetActorLocation) "0, 0, 0" 1.0 1.0 0.0 0 0 0 0)
  (CallFunction|NotifyOwnerforDestroy))

(event EventTick
  (params (DeltaSeconds :type Float%20%28single-precision%29))
  ;[1 1 1] BeginPlay & Destroy
  ;;[1 1 1] Tick: 0.05secs!
  (CallFunction|DestroyifOutsidetheViewport))

(fn ConstructionScript)

(fn PlayExplosionVFX
  (Game|SpawnActorfromClass "/Game/Blueprints/VFX/BP_Explosion_PlayerProjectile.BP_Explosion_PlayerProjectile_C" (Math|Transform|MakeTransform (Transformation|GetActorLocation) (Transformation|GetActorRotation) "1.000000,1.000000,1.000000") "AlwaysSpawn" "MultiplyWithRoot" 0 0))

(fn NotifyOwnerforDestroy
  (bind _returnvalue (Components|GetOwner))
  (if (Utilities|IsValid _returnvalue)
    (bind _asbpi_shoot (Utilities|Casting|CastToBPI_Shoot _returnvalue))
    (Default|NotifyBulletAbouttobeDestroyed _asbpi_shoot (Variables|Default|GetDamage))))

(fn DestroyifOutsidetheViewport
  (bind _returnvalue (Game|GetPlayerController 0))
  (bind _returnvalue_2 (Transformation|GetActorLocation))
  (bind _screenlocation (Class|PlayerController|ProjectWorldLocationtoScreen _returnvalue _returnvalue_2 false))
  (if (or (< (.x _screenlocation) 0.0) (> (.x _screenlocation) (.x (Viewport|GetViewportSize))))
    (Actor|DestroyActor)))