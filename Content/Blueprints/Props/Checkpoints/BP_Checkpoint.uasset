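; BP_Checkpoint is a fountain checkpoint prop that registers itself as the active checkpoint when the player reaches it.
; On BeginPlay it caches BP_PlayerGameMode, and the construction script assigns the fountain tile map.
; The collision box overlap sets the game mode's CheckPoint to itself, activates Niagara and plays the pickup sound.
; A DoOnce gate precedes the BP_Player cast, so the first overlap by any actor consumes it.
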(event OnComponentBeginOverlap(CollisionBox)
  (params (OverlappedComponent :type Primitive%20Component%20Object%20Reference) (OtherActor :type Actor%20Object%20Reference) (OtherComp :type Primitive%20Component%20Object%20Reference) (OtherBodyIndex :type Integer) (bFromSweep :type Boolean) (SweepResult :type Hit%20Result%20Structure%20%28by%20ref%29))
  (Utilities|FlowControl|DoOnce false
    (:Completed
      (Utilities|Casting|CastToBP_Player OtherActor)
      (Variables|/Game/Blueprints/BP_PlayerGameMode.BP_PlayerGameMode_C|SetCheckPoint (Variables|Default|GetGameMode) self)
      (Components|Activation|Activate (Variables|Default|GetNiagara) false)
      (Audio|Components|Audio|Play (Variables|Default|GetCheckpointPickup) 0.0))))

(event EventBeginPlay
  (bind _asbp_player_game_mode (Utilities|Casting|CastToBP_PlayerGameMode (Game|GetGameMode)))
  (Variables|Default|SetGameMode _asbp_player_game_mode))

(fn ConstructionScript
  (Class|PaperTileMapComponent|SetTileMap (Variables|Default|GetFountainTileMap) "/Game/Blueprints/Props/Checkpoints/TM_CheckpointFountain.TM_CheckpointFountain"))