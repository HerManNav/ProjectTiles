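; BP_PlayerGameMode is a game mode that handles player spawning at a checkpoint and caps the frame rate.
; BeginPlay runs the parent logic, then sets t.maxfps to 120 by console command.
; SpawnPlayer spawns the default pawn at the CheckPoint actor's location and rotation, then has player controller 0 possess it.
; HUD creation and the enemy transform reset loop are unconnected, leaving ResetAllEnemiesTransforms empty.
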(event EventBeginPlay
  (|CallParentFunction)
  (Utilities|FlowControl|Sequence
    (:then_0
      (Development|ExecuteConsoleCommand "t.maxfps 120" 0))
    (:then_1)))

(fn ConstructionScript)

(fn SpawnPlayer
  (bind _checkpoint (Variables|Default|GetCheckPoint))
  (bind _returnvalue (Transformation|GetActorTransform _checkpoint))
  (bind _returnvalue_2 (Game|SpawnActorfromClass (Variables|Default|GetDefaultPawnClass) (Math|Transform|MakeTransform (.location _returnvalue) (.rotation _returnvalue) "1.000000,1.000000,1.000000") "AdjustIfPossibleButAlwaysSpawn" "MultiplyWithRoot" 0 0))
  (Pawn|Possess (Game|GetPlayerController 0) _returnvalue_2))

(fn ResetAllEnemiesTransforms)